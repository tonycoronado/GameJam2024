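; Snowman enemy that turns toward the player and fires snowballs while the player is inside its AimZone trigger.
; Overlap starts a looping timer that smoothly interpolates yaw toward the player character cached at BeginPlay.
; A self-repeating Delay loop re-arms aiming and spawns SnowBall_BP at the Spawn component.
; Leaving clears the timer and flag, but the loop keeps cycling, with the flag gating rotation and shots.
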(event OnComponentBeginOverlap(AimZone)
  (params (OverlappedComponent :type Primitive%20Component%20Object%20Reference) (OtherActor :type Actor%20Object%20Reference) (OtherComp :type Primitive%20Component%20Object%20Reference) (OtherBodyIndex :type Integer) (bFromSweep :type Boolean) (SweepResult :type Hit%20Result%20Structure%20%28by%20ref%29))
  (Utilities|Casting|CastToBP_Player OtherActor)
  (Variables|Default|SetAimZone? true)
  (Utilities|FlowControl|Sequence :!label _label
    (:then_0
      (CallFunction|Aim))
    (:then_1
      (CallFunction|Shot)
      (Utilities|FlowControl|Delay (Variables|Default|GetShottoAim))
      (goto _label))))

(event OnComponentEndOverlap(AimZone)
  (params (OverlappedComponent :type Primitive%20Component%20Object%20Reference) (OtherActor :type Actor%20Object%20Reference) (OtherComp :type Primitive%20Component%20Object%20Reference) (OtherBodyIndex :type Integer))
  (Utilities|Casting|CastToBP_Player OtherActor)
  (Utilities|Time|ClearandInvalidateTimerbyHandle (Variables|Default|GetTimerHolder))
  (Variables|Default|SetAimZone? false))

(event Custom|Shot
  ;[0.15 0.15 0.15 0.5] Shot
  (if (Variables|Default|GetAimZone?)
    (Development|PrintString "Shot")
    (Game|SpawnActorfromClass "/Game/Marcel/AI/SnowBall_BP.SnowBall_BP_C" (Transformation|GetWorldTransform (Variables|Default|GetSpawn)) "Undefined" "MultiplyWithRoot" 0 0)))

(event Custom|Rote
  ;[0.15 0.15 0.15 0.5] Aim
  (if (Variables|Default|GetAimZone?)
    (Transformation|SetActorRotation (Math|Rotator|MakeRotator 0.0 0.0 (.yaw (Math|Interpolation|RInterpTo (Transformation|GetActorRotation) (Math|Rotator|FindLookatRotation (Transformation|GetActorLocation) (Transformation|GetActorLocation (Variables|Default|GetREF))) (Utilities|Time|GetWorldDeltaSeconds) (Variables|Default|GetInterp%20Speed)))))))

(event Custom|Aim
  ;[0.15 0.15 0.15 0.5] Aim
  (bind _returnvalue (Utilities|Time|SetTimerbyEvent (delegate Custom|Rote) 0.01 true true))
  (Variables|Default|SetTimerHolder _returnvalue))

(event EventBeginPlay
  (bind _asbp_player (Utilities|Casting|CastToBP_Player (Game|GetPlayerCharacter 0)))
  (Variables|Default|SetREF _asbp_player))

(event Collision|EventActorBeginOverlap
  (params (OtherActor :type Actor%20Object%20Reference)))

(event EventTick
  (params (DeltaSeconds :type Float%20%28single-precision%29)))

(fn ConstructionScript)