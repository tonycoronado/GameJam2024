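; Wave spawner that places random pickups and snowmen at marker actors in the level when HandleSpawning receives the amounts.
; BeginPlay gathers the pickup and snowman point actors, and random picks remove used points to avoid repeats.
; Each call restores all pickup points, destroys earlier pickups and gives new ones a reference to the spawner.
; The snowman point pool is not refilled here, so it shrinks across calls.
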(event Custom|HandleSpawning
  (params (PickupAmount :type Integer) (SnowmenAmount :type Integer))
  (Variables|Default|SetAvaiablePSP (Variables|Default|GetPickupSpawnPoints))
  (CallFunction|SpawnPickups PickupAmount)
  (CallFunction|SpawnSnowmen SnowmenAmount))

(event EventBeginPlay
  (bind _outactors (Actor|GetAllActorsOfClass "/Game/Max/Blueprints/Pickups/Spawner/BP_SnowmanPoint.BP_SnowmanPoint_C"))
  (Variables|Default|SetAvaiableSSP _outactors)
  (bind _outactors_2 (Actor|GetAllActorsOfClass "/Game/Max/Blueprints/Pickups/Spawner/BP_PickupPoint.BP_PickupPoint_C"))
  (Variables|Default|SetPickupSpawnPoints _outactors_2))

(fn ConstructionScript)

(fn SpawnPickups
  (params (LastIndex :type Integer))
  (for _array_element (Variables|Default|GetSpawnedPickups)
    (Utilities|IsValid _array_element
      (:Is%20Valid
        (Actor|DestroyActor _array_element))))
  (for _index (range 1 LastIndex)
    (bind _output_get (LocalVariables|SetSpawnPoint (.OutItem (Utilities|Array|Random (Variables|Default|GetAvaiablePSP)))))
    (bind _returnvalue (Game|SpawnActorfromClass (.OutItem (Utilities|Array|Random (Variables|Default|GetPickups))) (Transformation|GetActorTransform _output_get) "Undefined" "MultiplyWithRoot" 0 0))
    (bind _output_get_2 (LocalVariables|SetPickup _returnvalue))
    (Variables|/Game/Max/Blueprints/Pickups/BP_PickupBase.BP_PickupBase_C|SetSpawner _output_get_2 self)
    (Utilities|Array|Add (Variables|Default|GetSpawnedPickups) (LocalVariables|GetPickup))
    (Utilities|Array|RemoveItem (Variables|Default|GetAvaiablePSP) (LocalVariables|GetSpawnPoint))))

(fn SpawnSnowmen
  (params (LastIndex :type Integer))
  (for _index (range 1 LastIndex)
    (bind _output_get (LocalVariables|SetSpawnPoint (.OutItem (Utilities|Array|Random (Variables|Default|GetAvaiableSSP)))))
    (Utilities|IsValid _output_get
      (:Is%20Valid
        (Game|SpawnActorfromClass "/Game/Marcel/AI/Snowman_BP.Snowman_BP_C" (Transformation|GetActorTransform _output_get) "Undefined" "MultiplyWithRoot" 0 0)
        (Utilities|Array|RemoveItem (Variables|Default|GetAvaiableSSP) (LocalVariables|GetSpawnPoint))))))