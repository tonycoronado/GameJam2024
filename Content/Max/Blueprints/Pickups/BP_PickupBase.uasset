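; BP_PickupBase is a base pickup actor that is collected when the player character touches it.
; Its Sphere component's begin-overlap checks the other actor against player character 0 and calls the PickUp event.
; PickUp removes the pickup from its Spawner's SpawnedPickups collection, then destroys the actor.
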(event OnComponentBeginOverlap(Sphere)
  (params (OverlappedComponent :type Primitive%20Component%20Object%20Reference) (OtherActor :type Actor%20Object%20Reference) (OtherComp :type Primitive%20Component%20Object%20Reference) (OtherBodyIndex :type Integer) (bFromSweep :type Boolean) (SweepResult :type Hit%20Result%20Structure%20%28by%20ref%29))
  (if (== OtherActor (Game|GetPlayerCharacter 0))
    (Default|PickUp self)))

(event EventBeginPlay)

(event Collision|EventActorBeginOverlap
  (params (OtherActor :type Actor%20Object%20Reference)))

(event EventTick
  (params (DeltaSeconds :type Float%20%28single-precision%29)))

(event EventPickUp
  (Utilities|Array|RemoveItem (Variables|/Game/Max/Blueprints/Pickups/Spawner/BP_WaveSpawner.BP_WaveSpawner_C|GetSpawnedPickups (Variables|Default|GetSpawner)) self)
  (Actor|DestroyActor))

(fn ConstructionScript)