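; BP_Speedup is a pickup that gives the player a timed speed boost when collected.
; On PickUp it plays a 2D power-up sound, then passes its boost amount, duration and an effect type to BP_Player's OnSpeedEffect.
; It then calls the parent PickUp; if the player cast fails, both the boost and that parent call are skipped.
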(event EventBeginPlay
  (|CallParentFunction) ; This node is disabled and will not be called.\nDrag off pins to build functionality.
)

(event Collision|EventActorBeginOverlap
  (params (OtherActor :type Actor%20Object%20Reference))
  (|CallParentFunction OtherActor) ; This node is disabled and will not be called.\nDrag off pins to build functionality.
)

(event EventTick
  (params (DeltaSeconds :type Float%20%28single-precision%29))
  (|CallParentFunction DeltaSeconds) ; This node is disabled and will not be called.\nDrag off pins to build functionality.
)

(event EventPickUp
  (Audio|PlaySound2D "/Game/Marcel/Sounds/GetPowerUp.GetPowerUp" 1.0 1.0 0.0 0 0)
  (bind _asbp_player (Utilities|Casting|CastToBP_Player (Game|GetPlayerCharacter 0)))
  (Default|OnSpeedEffect _asbp_player (Variables|Default|GetBoostAmount) (Variables|Default|GetBoostTime) "NewEnumerator0")
  (|CallParentFunction))

(fn ConstructionScript
  (|CallParentFunction))