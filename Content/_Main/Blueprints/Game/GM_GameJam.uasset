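; Game mode for a wave-based gift delivery game, handling wave flow, countdown, pause and game over.
; BeginPlay copies DT_WavesData rows into WavesInfo, then StartGame spawns pickups and snowmen through BP_WaveSpawner, activates delivery zones and updates the HUD.
; A looping one-second timer decrements the wave's seconds directly in WavesInfo, ending the game at zero.
; PlayNextWave increments the wave, makes an extra fixed-count spawn, then restarts via StartGame after delays.
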(event Custom|Play%20Next%20Wave
  (bind _result (Math|Integer|IncrementInt (Variables|Default|GetWaveCount))
    (:%20%20
      ;[0.15 0 0 0.5] Max Code Function
      (Default|HandleSpawning (Variables|Default|GetWave%20Spawner) 2 2)
      (Utilities|FlowControl|Delay 5.0)
      (Default|PrepareMessage (Variables|Default|GetHUDRef))
      (Utilities|FlowControl|Delay 3.0)
      (CallFunction|StartGame))))

(event Custom|Start%20Game
  (bind _wavecount (Variables|Default|GetWaveCount))
  (bind _wavesinfo (Variables|Default|GetWavesInfo))
  (bind _output (Utilities|Array|Get(acopy) _wavesinfo _wavecount))
  (bind (_goalgifts _seconds _numberofsnowman _numberofpickups) (Utilities|Struct|BreakS_WavesInfo _output))
  (bind _returnvalue (Actor|GetActorOfClass "/Game/_Main/Blueprints/Gifts/BP_Gift_Master.BP_Gift_Master_C"))
  (Default|EnablePickupGift _returnvalue)
  (Default|HandleSpawning (Variables|Default|GetWave%20Spawner) _numberofpickups _numberofsnowman)
  (Default|UpdateGiftScore (Variables|/Game/_Main/Blueprints/Game/HUD_GameJam.HUD_GameJam_C|GetHud%20widget%20Ref (Variables|Default|GetHUDRef)) (Utilities|Text|ToText(Integer) _goalgifts))
  (Default|UpdateTime (Variables|/Game/_Main/Blueprints/Game/HUD_GameJam.HUD_GameJam_C|GetHud%20widget%20Ref (Variables|Default|GetHUDRef)) (Utilities|Text|ToText(Integer) _seconds))
  (Default|UpdateWaveCounter (Variables|/Game/_Main/Blueprints/Game/HUD_GameJam.HUD_GameJam_C|GetHud%20widget%20Ref (Variables|Default|GetHUDRef)) (Utilities|Text|ToText(Integer) (+ (Variables|Default|GetWaveCount) 1)))
  (bind _outactors (Actor|GetAllActorsOfClass "/Game/_Main/Blueprints/Gifts/BP_DeliveryZone_Master.BP_DeliveryZone_Master_C"))
  (for _array_element _outactors
    (Default|ActivateZone _array_element))
  (CallFunction|StartTimer)
  (Variables|Default|SetbWaveInProgress true))

(event Custom|Start%20Timer
  ;[0.15 0.15 0.15 0.5] Clock
  (bind _returnvalue (Utilities|Time|SetTimerbyFunctionName 0 "Timer Countdown" 1.0 true))
  (Variables|Default|SetTimer%20Handle _returnvalue))

(event Custom|Handle%20Pause%20Game
  (if (not (Variables|Default|GetGameFinished))
    (if (Game|IsGamePaused)
      (Game|SetGamePaused false)
      (else
        (Game|SetGamePaused true)
        (Default|PauseGameScreen (Variables|Default|GetHUDRef))))))

(event Custom|Stop%20Timer
  ;[0.15 0.15 0.15 0.5] Clock
  (Utilities|Time|ClearandInvalidateTimerbyHandle (Variables|Default|GetTimer%20Handle)))

(event Custom|Quit%20Game
  (CallFunction|QuitGame))

(event Custom|Pause%20Timer
  ;[0.15 0.15 0.15 0.5] Clock
  (Utilities|Time|PauseTimerbyHandle (Variables|Default|GetTimer%20Handle)))

(event Custom|Game%20Over
  (bind _returnvalue (Game|SetGamePaused true))
  (Variables|Default|SetGameFinished _returnvalue)
  (Default|GameOverScreen (Variables|Default|GetHUDRef))
  (CallFunction|StopTimer))

(event Custom|Unpause%20Timer
  ;[0.15 0.15 0.15 0.5] Clock
  (Utilities|Time|UnpauseTimerbyHandle (Variables|Default|GetTimer%20Handle)))

(event EventBeginPlay
  (Utilities|FlowControl|Sequence
    (:then_0
      (bind _hudref (Class|BPIGetRefs|GetHudRef(Message) (HUD|GetHUD (Game|GetPlayerController 0))))
      (Variables|Default|SetHUDRef _hudref)
      (Variables|Default|SetWaveCount 0)
      ;[0.15 0.15 0.15 0.5] Pass Data from Data Table to Struct
      (bind _outrownames (DataTable|GetDataTableRowNames "/Game/_Main/Blueprints/Game/Data/DT_WavesData.DT_WavesData"))
      (for (_array_element _array_index) _outrownames
        (bind _returnvalue (Utilities|GetDataTableRow "/Game/_Main/Blueprints/Game/Data/DT_WavesData.DT_WavesData" _array_element)
          (:then
            (Utilities|Array|SetArrayElem (Variables|Default|GetWavesInfo) _array_index (Utilities|Struct|MakeS_WavesInfo (.GoalGifts (Utilities|Struct|BreakS_WavesInfo _returnvalue)) (.Seconds (Utilities|Struct|BreakS_WavesInfo _returnvalue)) (.NumberOfSnowman (Utilities|Struct|BreakS_WavesInfo _returnvalue)) (.NumberOfPickups (Utilities|Struct|BreakS_WavesInfo _returnvalue))))))))
    (:then_1
      (bind _returnvalue_2 (Actor|GetActorOfClass "/Game/Max/Blueprints/Pickups/Spawner/BP_WaveSpawner.BP_WaveSpawner_C"))
      (Variables|Default|SetWave%20Spawner _returnvalue_2)
      (Utilities|FlowControl|Delay 2.0)
      (Default|PrepareMessage (Variables|Default|GetHUDRef))
      (Utilities|FlowControl|Delay 3.0)
      (CallFunction|StartGame))))

(fn ConstructionScript)

(fn TimerCountdown
  (bind _wavesinfo (Variables|Default|GetWavesInfo))
  (bind _wavecount (Variables|Default|GetWaveCount))
  (bind _output (Utilities|Array|Get(acopy) _wavesinfo _wavecount))
  (bind (_goalgifts _seconds _numberofsnowman _numberofpickups) (Utilities|Struct|BreakS_WavesInfo _output))
  (bind _output_get (LocalVariables|SetRemaining%20Seconds (- _seconds 1)))
  (Utilities|Array|SetArrayElem (Variables|Default|GetWavesInfo) (Variables|Default|GetWaveCount) (Utilities|Struct|MakeS_WavesInfo _goalgifts _output_get _numberofsnowman _numberofpickups))
  (bind _hudref (Class|BPIGetRefs|GetHudRef(Message) (HUD|GetHUD (Game|GetPlayerController 0))))
  (Default|UpdateTime (Variables|/Game/_Main/Blueprints/Game/HUD_GameJam.HUD_GameJam_C|GetHud%20widget%20Ref _hudref) (Utilities|Text|ToText(Integer) (LocalVariables|GetRemaining%20Seconds)))
  (if (<= (LocalVariables|GetRemaining%20Seconds) 0)
    (CallFunction|GameOver))
  (return))

(fn GetGameModeRef
  (return self))

(fn GetHudRef
  (return 0))