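; HUD_GameJam is the game jam HUD Blueprint that creates and shows the game's screen widgets for player 0.
; BeginPlay creates WBP_HUD and adds it to the viewport, storing a reference.
; Separate events open the pause and game over widgets; game over also shows the mouse cursor and switches input to UI only.
; GetHudRef returns the HUD itself, while GetGameModeRef returns nothing.
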(event Custom|Start%20Initial%20Info%20Widget
  (bind _returnvalue (UserInterface|CreateWidget "/Game/_Main/UI/WBP_HUD.WBP_HUD_C" (Game|GetPlayerController 0)))
  (bind _output_get (Variables|Default|SetHud%20widget%20Ref _returnvalue))
  (UserInterface|Viewport|AddtoViewport _output_get 0))

(event Custom|Pause%20Game%20Screen
  (bind _returnvalue (UserInterface|CreateWidget "/Game/Marcel/UI/Pause/Pause_WB.Pause_WB_C" (Game|GetPlayerController 0)))
  (bind _output_get (Variables|Default|SetPauseWidget _returnvalue))
  (UserInterface|Viewport|AddtoViewport _output_get 0))

(event Custom|Game%20Over%20Screen
  (bind _returnvalue (Game|GetPlayerController 0))
  (bind _returnvalue_2 (UserInterface|CreateWidget "/Game/_Main/UI/WBP_GameOver.WBP_GameOver_C" (Game|GetPlayerController 0)))
  (bind _output_get (Variables|Default|SetGameOverWidget _returnvalue_2))
  (UserInterface|Viewport|AddtoViewport _output_get 0)
  (Variables|/Script/Engine.PlayerController|SetbShowMouseCursor _returnvalue true)
  (Input|SetInputModeUIOnly _returnvalue _returnvalue_2 "DoNotLock" false))

(event EventBeginPlay
  (CallFunction|StartInitialInfoWidget))

(fn ConstructionScript)

(fn GetGameModeRef
  (return 0))

(fn GetHudRef
  (return self))