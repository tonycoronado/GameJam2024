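; BP_DeliveryManager counts gift deliveries across the level and triggers the next wave once the required number is reached.
; On BeginPlay it binds to the gift-delivered event of every BP_DeliveryZone in the level.
; Each delivery increments a shared counter, which is never reset here, and an exact match with GiftsRequired calls PlayNextWave on GM_GameJam.
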(event Custom|Gift%20Delivered
  (Math|Integer|IncrementInt (Variables|Default|GetGiftsDelivered)
    (:%20%20
      (if (== (Variables|Default|GetGiftsDelivered) (Variables|Default|GetGiftsRequired))
        (bind _asgm_game_jam (Utilities|Casting|CastToGM_GameJam (Game|GetGameMode)))
        (Default|PlayNextWave _asgm_game_jam)))))

(event EventBeginPlay
  (bind _outactors (Actor|GetAllActorsOfClass "/Game/_Main/Blueprints/Gifts/BP_DeliveryZone.BP_DeliveryZone_C"))
  (for _array_element _outactors
    (EventDispatchers|BindEventtoOnGiftDeliveredatZone _array_element (delegate Custom|Gift%20Delivered))))

(fn ConstructionScript)