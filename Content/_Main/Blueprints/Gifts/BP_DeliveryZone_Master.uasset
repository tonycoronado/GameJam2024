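; Master delivery zone actor where gifts are dropped off, toggled active or inactive via sphere collision and a blue or red material.
; When an actor tagged Gift overlaps the sphere, it destroys the gift, deactivates itself, plays a delivery sound and fires OnGiftDeliveredAtZone.
; It then clears the player's has-gift state through BP_Player.
; BeginPlay caches the DeliveryManager, though this graph never uses it.
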(event OnComponentBeginOverlap(SphereCollision)
  (params (OverlappedComponent :type Primitive%20Component%20Object%20Reference) (OtherActor :type Actor%20Object%20Reference) (OtherComp :type Primitive%20Component%20Object%20Reference) (OtherBodyIndex :type Integer) (bFromSweep :type Boolean) (SweepResult :type Hit%20Result%20Structure%20%28by%20ref%29))
  (if (Actor|ActorHasTag OtherActor "Gift")
    (Actor|DestroyActor OtherActor)
    (CallFunction|DeactivateZone)
    (Audio|PlaySound2D "/Game/Marcel/Sounds/GIFTDELIVERY.GIFTDELIVERY" 1.0 1.0 0.0 0 0)
    (Default|CallOnGiftDeliveredatZone)
    (bind _returnvalue (Actor|GetActorOfClass "/Game/_Main/Blueprints/Player/BP_Player.BP_Player_C"))
    (Default|HandlePlayerHasGift _returnvalue false)))

(event Custom|Deactivate%20Zone
  (Collision|SetCollisionEnabled (Variables|Default|GetSphereCollision) "NoCollision")
  (Rendering|Material|SetMaterial (Variables|Default|GetMesh) 0 "/Game/LevelPrototyping/Materials/MI_Solid_Red.MI_Solid_Red"))

(event Custom|ActivateZone
  (Collision|SetCollisionEnabled (Variables|Default|GetSphereCollision) "QueryOnly")
  (Rendering|Material|SetMaterial (Variables|Default|GetMesh) 0 "/Game/LevelPrototyping/Materials/MI_Solid_Blue.MI_Solid_Blue"))

(event EventBeginPlay
  (bind _returnvalue (Actor|GetActorOfClass "/Game/_Main/Blueprints/Gifts/BP_DeliveryManager.BP_DeliveryManager_C"))
  (Variables|Default|SetDeliveryManager _returnvalue))

(fn ConstructionScript)